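; Game mode for the FallGuys game that drives the match through Ready, Play and End states held in BP_GameState.
; On BeginPlay it binds to the game state's change and TS dispatchers, then sets Ready, switching to Play once TS exceeds a five-unit threshold.
; OnGameEnd sets End, then gives the passed character's player state one result and every other BP_PlayerState the other.
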(event EventBeginPlay
  (bind _asbp_game_state (Utilities|Casting|CastToBP_GameState (Game|GetGameState)))
  (EventDispatchers|BindEventtoEventDispatcherChangeGameState _asbp_game_state (EventDispatchers|CreateEvent :!event EventChangeGameState))
  (EventDispatchers|BindEventtoEventDispatcherTS _asbp_game_state (EventDispatchers|CreateEvent :!event EventTS))
  (bind _asbp_game_state_2 (Utilities|Casting|CastToBP_GameState (Game|GetGameState)))
  (Default|ChangeGameState _asbp_game_state_2 "NewEnumerator1"))

(fn ConstructionScript)

(fn EventChangeGameState
  (params (GameState :type EN_GameState%20Enum :default "NewEnumerator0"))
  (Variables|Default|SetGame%20State GameState))

(fn EventTS
  (params (TS :type Float%20%28double-precision%29))
  (switch Utilities|FlowControl|Switch|SwitchonEN_GameState (Variables|Default|GetGame%20State)
    (:NewEnumerator1
      (if (> TS 5.0)
        (bind _asbp_game_state (Utilities|Casting|CastToBP_GameState (Game|GetGameState)))
        (Default|ChangeGameState _asbp_game_state "NewEnumerator2")))))

(fn OnGameEnd
  (params (Character :type Character%20Object%20Reference))
  (bind _asbp_game_state (Utilities|Casting|CastToBP_GameState (Game|GetGameState)))
  (Default|ChangeGameState _asbp_game_state "NewEnumerator3")
  (CallFunction|UpdatePlayerResult (Variables|/Script/Engine.Pawn|GetPlayerState Character)))

(fn UpdatePlayerResult
  (params (Object :type Object%20Object%20Reference))
  (bind _asbp_player_state (Utilities|Casting|CastToBP_PlayerState Object))
  (Default|SetResult _asbp_player_state "NewEnumerator1")
  (bind _outactors (Actor|GetAllActorsOfClass "/Game/FallGuys/BP_PlayerState.BP_PlayerState_C"))
  (for _array_element _outactors
    (if (!= _array_element _asbp_player_state)
      (Default|SetResult _array_element "NewEnumerator2"))))