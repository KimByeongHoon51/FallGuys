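; Game state Blueprint for a Fall Guys-style game that tracks the current phase and the time elapsed in it.
; Tick runs a handler for the Ready or Play phase, where only the authority accumulates time, then every instance broadcasts the total through the TS dispatcher.
; ChangeGameState sets the phase and resets the timer, and the phase's RepNotify broadcasts the new state through an event dispatcher.
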(event EventTick
  (params (DeltaSeconds :type Float%20%28single-precision%29))
  (switch Utilities|FlowControl|Switch|SwitchonEN_GameState (Variables|Default|GetGameState)
    (:NewEnumerator1
      (CallFunction|TickReady DeltaSeconds))
    (:NewEnumerator2
      (CallFunction|TickPlay DeltaSeconds))))

(fn ConstructionScript)

(fn ChangeGameState
  (params (GameState :type EN_GameState%20Enum :default "NewEnumerator0"))
  (Variables|Default|SetGameState GameState)
  (Variables|Default|SetTotalDeltaSec 0.0))

(fn OnRepGameState
  (Default|CallEventDispatcherChangeGameState (Variables|Default|GetGameState)))

(fn TickReady
  (params (DeltaSec :type Float%20%28double-precision%29))
  (Utilities|FlowControl|Sequence
    (:then_0
      (Networking|SwitchHasAuthority
        (:Authority
          (Variables|Default|SetTotalDeltaSec (+ (Variables|Default|GetTotalDeltaSec) DeltaSec)))))
    (:then_1
      (Default|CallEventDispatcherTS (Variables|Default|GetTotalDeltaSec)))))

(fn TickPlay
  (params (DeltaSec :type Float%20%28double-precision%29))
  (Utilities|FlowControl|Sequence
    (:then_0
      (Networking|SwitchHasAuthority
        (:Authority
          (Variables|Default|SetTotalDeltaSec (+ (Variables|Default|GetTotalDeltaSec) DeltaSec)))))
    (:then_1
      (Default|CallEventDispatcherTS (Variables|Default|GetTotalDeltaSec)))))