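; BP_Tile is a floor tile that destroys itself two seconds after a player character overlaps its box.
; The box starts with collision disabled, and BeginPlay binds to the BP_GameState change dispatcher, whose handler enables query and physics collision after a state comparison.
; The overlap response runs only on the authority, so the server controls the tile's removal.
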(event OnComponentBeginOverlap(Box)
  (params (OverlappedComponent :type Primitive%20Component%20Object%20Reference) (OtherActor :type Actor%20Object%20Reference) (OtherComp :type Primitive%20Component%20Object%20Reference) (OtherBodyIndex :type Integer) (bFromSweep :type Boolean) (SweepResult :type Hit%20Result%20Structure%20%28by%20ref%29))
  (Networking|SwitchHasAuthority
    (:Authority
      (Utilities|Casting|CastToBP_ThirdPersonCharacter OtherActor)
      (Utilities|FlowControl|Delay 2.0)
      (Actor|DestroyActor))))

(event EventBeginPlay
  (Collision|SetCollisionEnabled (Variables|Default|GetBox) "NoCollision")
  (bind _asbp_game_state (Utilities|Casting|CastToBP_GameState (Game|GetGameState)))
  (EventDispatchers|BindEventtoEventDispatcherChangeGameState _asbp_game_state (EventDispatchers|CreateEvent :!event ChangeGameState)))

(fn ConstructionScript)

(fn ChangeGameState
  (params (GameState :type EN_GameState%20Enum :default "NewEnumerator0"))
  (if (Utilities|Enum|Equal(Enum) GameState (Variables|Default|GetGameState))
    (Collision|SetCollisionEnabled (Variables|Default|GetBox) "QueryAndPhysics")))